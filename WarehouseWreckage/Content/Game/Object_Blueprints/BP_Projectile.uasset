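; BP_Projectile is a physics-driven projectile that launches itself on spawn and destroys itself after its Lifespan.
; BeginPlay prints the actor's display name, calls Launch, then waits out the delay before destruction.
; Launch applies a mass-independent velocity-change impulse to the static mesh, scaled by LaunchSpeed along player 0's controller forward vector rather than the projectile's own.
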(event EventBeginPlay
  (CallFunction|PrintName)
  (CallFunction|Launch)
  (Utilities|FlowControl|Delay (Variables|Default|GetLifespan))
  (Actor|DestroyActor))

(event Collision|EventActorBeginOverlap
  (params (OtherActor :type Actor%20Object%20Reference)))

(event EventTick
  (params (DeltaSeconds :type Float%20%28single-precision%29)))

(fn ConstructionScript)

(fn PrintName
  (Development|PrintString (Utilities|GetDisplayName self)))

(fn Launch
  (Physics|AddImpulse (Variables|/Script/Engine.StaticMeshActor|GetStaticMeshComponent self) (* (Math|Conversions|ToVector(Float) (Variables|Default|GetLaunchSpeed)) (Transformation|GetActorForwardVector (Pawn|GetController (Game|Player|GetPlayerPawn 0)))) "None" true))